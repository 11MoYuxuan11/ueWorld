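; RTS player commander that pans and zooms a spring-arm camera and starts unit selection from mouse input.
; Movement axes, combined with edge-axis variables, move the actor along camera yaw; a separate CameraMove function does screen-edge scrolling but is not called here.
; Left press records the cursor position, and a gated comparison tells click from drag to drive BP_RTSCameraHUD's selection box.
; Release, right-click orders, construction placement and ClearSelected are empty stubs.
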(event Custom|GoToPressed)

(event Custom|GoToReleased)

(event Custom|Place/Select%20Pressed
  (bind _returnvalue (Game|GetPlayerController 0))
  (bind _returnvalue_2 (Game|GetPlayerController 0))
  (bind (_locationx _locationy) (Game|Player|GetMousePosition _returnvalue))
  (bind (_locationx_2 _locationy_2) (Game|Player|GetMousePosition _returnvalue_2))
  (CallFunction|ClearSelected)
  (if (Variables|Default|GetConstructionMode)
    (if (Variables|Default|GetbInsufficientResource)
      _)
    (else
      (Variables|Default|SetClickedLocation (Math|Vector2D|MakeVector2D _locationx _locationy))
      (Utilities|FlowControl|Gate true ; enters at Open
        (:Exit
          ;[1 1 1] 判断位置变化，决定是否生成选框
          (if (and (== (.x (Variables|Default|GetClickedLocation)) _locationx_2) (== (.y (Variables|Default|GetClickedLocation)) _locationy_2))
            ;[1 1 1] 不绘制选择框
            (Variables|/Game/URTS/Core/BP_RTSCameraHUD.BP_RTSCameraHUD_C|SetbIsDrawing (Variables|Default|GetRef_HUD) false)
            (Variables|Default|SetSingleClick true)
            (else
              ;[1 1 1] 绘制选择框
              (Variables|/Game/URTS/Core/BP_RTSCameraHUD.BP_RTSCameraHUD_C|SetbIsDrawing (Variables|Default|GetRef_HUD) true)
              (Variables|/Game/URTS/Core/BP_RTSCameraHUD.BP_RTSCameraHUD_C|SetClickedLocation (Variables|Default|GetRef_HUD) (Variables|Default|GetClickedLocation))
              (Variables|Default|SetSingleClick false))))))))

(event Custom|Place/Released%20Released)

(event EventBeginPlay
  (bind _asbp_rtscamera_hud (Utilities|Casting|CastToBP_RTSCameraHUD (HUD|GetHUD (Game|GetPlayerController 0))))
  (Variables|Default|SetRef_HUD _asbp_rtscamera_hud))

(event Collision|EventActorBeginOverlap
  (params (OtherActor :type Actor%20Object%20Reference)))

(event EventTick
  (params (DeltaSeconds :type Float%20%28single-precision%29)))

(event Input|AxisEvents|InputAxisCameraZoom
  (params (AxisValue :type Float%20%28single-precision%29))
  (bind _springarm (Variables|Default|GetSpringArm))
  (if (!= AxisValue 0.0)
    (Variables|/Script/Engine.SpringArmComponent|SetTargetArmLength _springarm (+ (Variables|/Script/Engine.SpringArmComponent|GetTargetArmLength _springarm) (* 100 AxisValue)))))

(event Input|AxisEvents|InputAxisMoveForward
  (params (AxisValue :type Float%20%28single-precision%29))
  (Transformation|SetActorLocation (+ (Transformation|GetActorLocation) (* (Math|Vector|GetForwardVector (Math|Rotator|MakeRotator 0.0 0.0 (.yaw (Transformation|GetWorldRotation (Variables|Default|GetCamera))))) (* (+ AxisValue (Variables|Default|GetEdgeForwardAxis)) (Variables|Default|GetMovementSpeed)))) false false))

(event Input|AxisEvents|InputAxisMoveRight
  (params (AxisValue :type Float%20%28single-precision%29))
  (Transformation|SetActorLocation (+ (Transformation|GetActorLocation) (* (Math|Vector|GetRightVector (Math|Rotator|MakeRotator 0.0 0.0 (.yaw (Transformation|GetWorldRotation (Variables|Default|GetCamera))))) (* (+ AxisValue (Variables|Default|GetEdgeRightAxis)) (Variables|Default|GetMovementSpeed)))) false false))

(event Input|MouseEvents|RightMouseButton
  (params (Key :type Key%20Structure :default "None"))
  (:Pressed
    (CallFunction|GotoPressed))
  (:Released
    (CallFunction|GotoReleased)))

(event Input|MouseEvents|LeftMouseButton
  (params (Key :type Key%20Structure :default "None"))
  (:Pressed
    (CallFunction|Place/SelectPressed))
  (:Released
    (CallFunction|Place/ReleasedReleased)))

(fn ConstructionScript)

(fn CameraMove
  (bind _returnvalue (Viewport|GetViewportSize))
  (bind _returnvalue_2 (Class|WidgetLayoutLibrary|GetMousePositiononViewport))
  (Transformation|SetActorLocation (+ (Transformation|GetActorLocation) (* (+ (select (< (/ (.x _returnvalue_2) (.x _returnvalue)) 0.01) "0.000000,-1.000000, 0" "0, 0, 0") (select (> (/ (.x _returnvalue_2) (.x _returnvalue)) 0.99) "0,1.000000, 0" "0, 0, 0") (select (< (/ (.y _returnvalue_2) (.y _returnvalue)) 0.01) "1.000000,0.000000,0.000000" "0, 0, 0") (select (> (/ (.y _returnvalue_2) (.y _returnvalue)) 0.99) "-1.000000,0.000000,0.000000" "0, 0, 0")) 10)) false false)
  (return))

(fn ClearSelected)