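; BP_Chunk is a world chunk Blueprint that computes simplex-noise height values for terrain.
; CalculateNosie fills a Noise array over the chunk's square grid, offsetting samples by chunk index and flooring weighted 2D noise.
; GenerateHeight layers three offset 3D noise samples at different frequencies and decreasing amplitudes into one floored height.
; The events and construction script are empty, so neither function is called within this Blueprint.
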(event EventBeginPlay)

(event Collision|EventActorBeginOverlap
  (params (OtherActor :type Actor%20Object%20Reference)))

(event EventTick
  (params (DeltaSeconds :type Float%20%28single-precision%29)))

(fn ConstructionScript)

(fn CalculateNosie
  (bind _chunkelements (Variables|Default|GetchunkElements))
  (bind _returnvalue (- _chunkelements 1))
  (for _index (range 0 _returnvalue)
    (LocalVariables|SetYLoc _index)
    (for _index_2 (range 0 _returnvalue)
      (LocalVariables|SetXLoc _index_2)
      (bind _returnvalue_2 (Class|SimplexNoiseBPLibrary|SimplexNoise2D (* (+ (LocalVariables|GetXLoc) (* (Variables|Default|GetchunkXindex) (Variables|Default|GetchunkElements))) (Variables|Default|GetxMult)) (* (+ (* (Variables|Default|GetchunkYindex) (Variables|Default|GetchunkElements)) (LocalVariables|GetYLoc)) (Variables|Default|GetyMult))))
      (Utilities|Array|Add (LocalVariables|Getnoise) (Math|Float|Floor (* _returnvalue_2 (Variables|Default|Getweight))))))
  (return (LocalVariables|Getnoise)))

(fn GenerateHeight
  (params (wPos :type Vector :default "0, 0, 0"))
  (bind _offset0 (Variables|Default|Getoffset0))
  (bind _amplitude (Variables|Default|GetAmplitude))
  (bind _offset1 (Variables|Default|Getoffset1))
  (bind _offset2 (Variables|Default|Getoffset2))
  (bind (_rx _ry _rz) (|CollapseGraph_0_2 wPos _offset0))
  (bind (_rx_2 _ry_2 _rz_2) (|CollapseGraph_0_2_3 wPos _offset2))
  (bind (_rx_3 _ry_3 _rz_3) (|CollapseGraph_0_2_2 wPos _offset1))
  (bind _returnvalue (Class|SimplexNoiseBPLibrary|SimplexNoise3D _rx _ry _rz))
  (bind _returnvalue_2 (Class|SimplexNoiseBPLibrary|SimplexNoise3D (* 2 _rx_3) (* 2 _ry_3) (* 2 _rz_3)))
  (bind _returnvalue_3 (Class|SimplexNoiseBPLibrary|SimplexNoise3D (/ _rx_2 4.0) (/ _ry_2 4.0) (/ _rz_2 4.0)))
  (return (Math|Float|Floor (+ (* _returnvalue _amplitude) (/ (* _returnvalue_2 _amplitude) 2.0) (/ (* _returnvalue_3 _amplitude) 4.0)))))