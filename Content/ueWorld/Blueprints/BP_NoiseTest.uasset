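; BP_NoiseTest is a test actor that builds a bumpy, terrain-like grid of instanced static meshes from 2D simplex noise.
; The construction script runs nested loops over the grid, samples noise at each index scaled by NewVar0, and adds an instance at that cell.
; The noise value sets each instance's height.
; The event graph holds only disabled placeholder events, so nothing is scripted at runtime.
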(event EventBeginPlay)

(event Collision|EventActorBeginOverlap
  (params (OtherActor :type Actor%20Object%20Reference)))

(event EventTick
  (params (DeltaSeconds :type Float%20%28single-precision%29)))

(fn ConstructionScript
  (bind _newvar_0 (Variables|Default|GetNewVar_0))
  (for _index (range 0 100)
    (for _index_2 (range 0 100)
      (bind _returnvalue (Class|SimplexNoiseBPLibrary|SimplexNoise2D (* _index _newvar_0) (* _index_2 _newvar_0)))
      (Components|InstancedStaticMesh|AddInstance (Variables|Default|GetInstancedStaticMesh) (Math|Conversions|ToTransform(Vector) (Math|Vector|MakeVector (* _index 1e+02) (* _index_2 1e+02) (* _returnvalue 1e+02)))))))