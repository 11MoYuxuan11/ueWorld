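; Player controller that moves a selection cube to the grid cell under the mouse cursor.
; It spawns a BP_SelectCube on BeginPlay, then each Tick line-traces from the camera along the deprojected mouse direction, ignoring the player pawn.
; WorldPostion2CubePosition converts the impact point into a cube position for the selection cube, without checking whether the trace hit.
; Debug trace drawing and impact-point printing run every frame.
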(event EventBeginPlay
  (bind _returnvalue (Game|SpawnActorfromClass "/Game/ueWorld/Blueprints/BP_SelectCube.BP_SelectCube_C" (Math|Transform|MakeTransform "0, 0, 0") "AlwaysSpawn" 0 0))
  (Variables|Default|SetSelectCube _returnvalue))

(event EventTick
  (params (DeltaSeconds :type Float%20%28single-precision%29))
  (bind _returnvalue (Game|GetPlayerCameraManager 0))
  (bind _returnvalue_2 (Camera|GetCameraLocation _returnvalue))
  (bind _outhit (Collision|LineTraceByChannel _returnvalue_2 (+ _returnvalue_2 (* (.WorldDirection (Game|Player|ConvertMouseLocationToWorldSpace)) 2e+03)) "TraceTypeQuery1" false (Utilities|Array|MakeArray (Game|Player|GetPlayerPawn 0)) "ForOneFrame"))
  (Development|PrintString (Utilities|String|ToString(Vector) (+ (.ImpactPoint (Collision|BreakHitResult _outhit)) "0.000000,0.000000,0.000000")))
  (bind _returnvalue_3 (Class|CubeMetrics|WorldPostion2CubePosition (+ (.ImpactPoint (Collision|BreakHitResult _outhit)) "0.000000,0.000000,0.000000") 1e+02))
  (Transformation|SetActorLocation (Variables|Default|GetSelectCube) _returnvalue_3 false false))

(fn ConstructionScript)