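; Voxel world manager that streams ChunkTest actors on an XY grid around the player pawn.
; Each tick it updates the player's position and chunk index, destroys chunks failing CheckRadius, then spawns missing passing ones within RenderRange.
; Parallel coordinate and actor arrays track live chunks.
; CheckRadius contains a player-distance test that is left unconnected, and ChunkSizeHalf actually equals the full chunk size.
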(event EventBeginPlay
  (CallFunction|Initialize))

(event EventTick
  (params (DeltaSeconds :type Float%20%28single-precision%29))
  (CallFunction|UpdatePosition)
  (CallFunction|RemoveChunk)
  (CallFunction|AddChunk))

(fn ConstructionScript)

(fn UpdatePosition
  (bind _chunksizehalf (Variables|Default|GetchunkSizeHalf))
  (bind _output_get (Variables|Default|SetcharacterPosition (* (Transformation|GetActorLocation (Game|Player|GetPlayerPawn 0)) "1.000000,1.000000, 0")))
  (if (or (!= (Variables|Default|GetchunkX) (Math|Float|Truncate (/ (.X (Math|Vector|BreakVector _output_get)) (Math|Conversions|ToFloat(Integer) _chunksizehalf)))) (!= (Variables|Default|GetchunkY) (Math|Float|Truncate (/ (.Y (Math|Vector|BreakVector _output_get)) (Math|Conversions|ToFloat(Integer) _chunksizehalf)))))
    (Variables|Default|SetchunkX (Math|Float|Truncate (/ (.X (Math|Vector|BreakVector _output_get)) (Math|Conversions|ToFloat(Integer) _chunksizehalf))))
    (Variables|Default|SetchunkY (Math|Float|Truncate (/ (.Y (Math|Vector|BreakVector _output_get)) (Math|Conversions|ToFloat(Integer) _chunksizehalf))))
    (return true)
    (else
      (return false))))

(fn Initialize
  (bind _output_get (Variables|Default|SetchunkSize (* (Variables|Setting|GetchunkLineElement) (Variables|Setting|GetvoxelSize))))
  (Variables|Default|SetchunkSizeHalf (/ _output_get 1)))

(fn AddChunk
  (bind _chunksize (Variables|Default|GetchunkSize))
  (bind _renderrange (Variables|Setting|GetrenderRange))
  (bind _chunkcords (Variables|Default|GetchunkCords))
  (bind _chunksizehalf (Variables|Default|GetchunkSizeHalf))
  (bind _returnvalue (Math|Conversions|ToFloat(Integer) _chunksize))
  (bind _returnvalue_2 (Math|Conversions|ToFloat(Integer) _chunksizehalf))
  (bind _returnvalue_3 (* _renderrange -1))
  (for _index (range _returnvalue_3 _renderrange) ; X
    (for _index_2 (range _returnvalue_3 _renderrange) ; Y
      (if (Utilities|CheckRadius (+ (* (+ _index (Variables|Default|GetchunkX)) _returnvalue) _returnvalue_2) (+ (* (+ _index_2 (Variables|Default|GetchunkY)) _returnvalue) _returnvalue_2))
        (if (not (Utilities|Array|ContainsItem _chunkcords (Math|Vector2D|MakeVector2D (Math|Conversions|ToFloat(Integer) (+ _index (Variables|Default|GetchunkX))) (Math|Conversions|ToFloat(Integer) (+ _index_2 (Variables|Default|GetchunkY))))))
          (Utilities|Array|Add _chunkcords (Math|Vector2D|MakeVector2D (Math|Conversions|ToFloat(Integer) (+ _index (Variables|Default|GetchunkX))) (Math|Conversions|ToFloat(Integer) (+ _index_2 (Variables|Default|GetchunkY)))))
          (bind _returnvalue_4 (Game|SpawnActorfromClass "/Game/ueWorld/Blueprints/ChunkTest.ChunkTest_C" (Math|Conversions|ToTransform(Vector) (Math|Vector|MakeVector (* (+ _index (Variables|Default|GetchunkX)) _returnvalue) (* (+ _index_2 (Variables|Default|GetchunkY)) _returnvalue) 0.0)) "Undefined" 0 0 (Variables|Setting|GetvoxelSize) (Variables|Setting|GetchunkLineElement) _index _index_2 0))
          (Utilities|Array|Add (Variables|Default|GetChunks) _returnvalue_4))))))

(fn RemoveChunk
  (bind _chunksize (Variables|Default|GetchunkSize))
  (bind _chunksizehalf (Variables|Default|GetchunkSizeHalf))
  (bind _chunks (Variables|Default|GetChunks))
  (bind _returnvalue (Math|Conversions|ToFloat(Integer) _chunksizehalf))
  (for (_array_element _array_index) (Variables|Default|GetchunkCords)
    (if (not (Utilities|CheckRadius (+ (* _chunksize (.X (Math|Vector2D|BreakVector2D _array_element))) _returnvalue) (+ (* _chunksize (.Y (Math|Vector2D|BreakVector2D _array_element))) _returnvalue)))
      (Actor|DestroyActor (Utilities|Array|Get(acopy) _chunks _array_index))
      (Utilities|Array|RemoveIndex (Variables|Default|GetchunkCords) _array_index)
      (Utilities|Array|RemoveIndex _chunks _array_index))))