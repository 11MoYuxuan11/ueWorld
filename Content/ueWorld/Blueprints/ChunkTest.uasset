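; ChunkTest is a test Blueprint for noise-based terrain chunks.
; CalculateNosie loops over a square of ChunkElements, samples 2D simplex noise at chunk-index-offset coordinates, and appends floored, weighted heights to the Noise array; its return node is unconnected.
; An older construction-script loop placing mesh instances at noise heights is disconnected.
; The event graph is empty, and nothing here calls CalculateNosie.
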(event EventBeginPlay)

(event Collision|EventActorBeginOverlap
  (params (OtherActor :type Actor%20Object%20Reference)))

(event EventTick
  (params (DeltaSeconds :type Float%20%28single-precision%29)))

(fn ConstructionScript)

(fn CalculateNosie
  (bind _chunkelements (Variables|Default|GetchunkElements))
  (bind _returnvalue (- _chunkelements 1))
  (for _index (range 0 _returnvalue)
    (LocalVariables|SetYLoc _index)
    (for _index_2 (range 0 _returnvalue)
      (LocalVariables|SetXLoc _index_2)
      (bind _returnvalue_2 (Class|SimplexNoiseBPLibrary|SimplexNoise2D (* (+ (LocalVariables|GetXLoc) (* (Variables|Default|GetchunkXindex) (Variables|Default|GetchunkElements))) (Variables|Default|GetxMult)) (* (+ (* (Variables|Default|GetchunkYindex) (Variables|Default|GetchunkElements)) (LocalVariables|GetYLoc)) (Variables|Default|GetyMult))))
      (Utilities|Array|Add (LocalVariables|Getnoise) (Math|Float|Floor (* _returnvalue_2 (Variables|Default|Getweight)))))))