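; Player character Blueprint with a modular body, Gameplay Ability System hooks and a main HUD.
; On BeginPlay, gear, hair and face components follow the main Mesh through master pose, and W_MainHUD is added to the viewport.
; Health changes update the HUD bar as a fraction of max health.
; Q tries to activate GA_DamageBase, printing the result, and inventory changes print the item name.
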(event OnInventoryItemChanged(Inventory)
  (params (bAdded :type Boolean) (Item :type Item%20Data%20Asset%20Object%20Reference))
  (Development|PrintText (Variables|/Script/InventorySystem.ItemDataAsset|GetItemName Item)))

(event Custom|UpdateHealthBar
  (Default|SetHPBar (Variables|Default|GetW_MainHUD) (/ (Class|UnWorldCharacter|GetHealth) (Class|UnWorldCharacter|GetMaxHealth))))

(event EventBeginPlay
  (Class|SkinnedMeshComponent|SetMasterPoseComponent (Variables|Default|GetHair) (Variables|Character|GetMesh) false)
  (bind _returnvalue (UserInterface|CreateWidget "/Game/unWorld/Widgets/W_MainHUD.W_MainHUD_C"))
  (bind _output_get (Variables|Default|SetW_MainHUD _returnvalue))
  (UserInterface|Viewport|AddtoViewport _output_get 0)
  (CallFunction|UpdateHealthBar))

(event EventOnHealthChanged
  (params (DeltaValue :type Float%20%28single-precision%29) (EventTags :type Gameplay%20Tag%20Container%20Structure%20%28by%20ref%29))
  (CallFunction|UpdateHealthBar))

(event EventTick
  (params (DeltaSeconds :type Float%20%28single-precision%29)))

(event Input|KeyboardEvents|Q
  (params (Key :type Key%20Structure :default "None"))
  (:Pressed
    (bind _returnvalue (Abilities|TryActivateAbilitybyClass (Variables|Default|GetAbilitySystemComponent) "/Game/unWorld/Abilities/GA_DamageBase.GA_DamageBase_C" true))
    (if _returnvalue
      (Development|PrintString "q")
      (else
        (Development|PrintString "not")))))

(fn ConstructionScript)