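; BP_CharacterBase is a character base Blueprint providing shared ability-state checks and montage playback.
; CanUseAnyAbility requires IsAlive (health above zero) and no active skill, though IsUsingSkill and IsUsingMelee are stubs returning false.
; PlayHighPriorityMontage stores and plays the given montage from a start section unless that montage is already playing.
; The event graph and construction script contain no logic.
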(event EventBeginPlay)

(event Collision|EventActorBeginOverlap
  (params (OtherActor :type Actor%20Object%20Reference)))

(event EventTick
  (params (DeltaSeconds :type Float%20%28single-precision%29)))

(fn ConstructionScript)

(fn CanUseAnyAbility
  (return (and (CallFunction|IsAlive) (not (CallFunction|IsUsingSkill)))))

(fn IsUsingSkill
  (return false))

(fn IsAlive
  (return (> (Class|UnWorldCharacter|GetHealth) 0.0)))

(fn PlayHighPriorityMontage
  (params (Montage :type Anim%20Montage%20Object%20Reference) (StartSectionName :type Name))
  (if (not (Animation|Montage|MontageIsPlaying (Components|SkeletalMesh|GetAnimInstance (Variables|Character|GetMesh)) Montage))
    (bind _output_get (Variables|Default|SetHighPriorityMontage Montage))
    (Animation|PlayAnimMontage _output_get 1.0 StartSectionName)))

(fn IsUsingMelee
  (return false))