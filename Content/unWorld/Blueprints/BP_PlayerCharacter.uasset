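; Player character Blueprint with modular body and gear meshes that follow the main mesh through master pose, plus an HP HUD and an inventory component.
; Slotted weapon items drive ChangeWeapon, which replaces the socket-attached weapon actor and swaps its attack ability in GameplayAbilities.
; Rolls play a high-priority montage, turning to control rotation when there is move input.
; Q test-fires GA_DamageBase, SimpleAttack plays a montage, and DoMeleeAttack only runs checks.
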(event OnSlottedItemChanged(Bpc_Inventory)
  (params (Slot :type Item%20Slot%20Structure) (Item :type Item%20Data%20Asset%20Object%20Reference))
  (if (== (.ItemType (Utilities|Struct|BreakItemSlot Slot)) "Weapon")
    (bind _asweapon_item_data (Utilities|Casting|CastToWeaponItemData Item))
    (bind _asbp_weapon_base (Utilities|Casting|CastToBP_WeaponBaseClass (Variables|/Script/InventorySystem.WeaponItemData|GetWeaponActor _asweapon_item_data)))
    (CallFunction|ChangeWeapon _asbp_weapon_base)))

(event Custom|UpdateHealthBar
  (Default|SetHPBar (Variables|Default|GetW_MainHUD) (/ (Class|UnWorldCharacter|GetHealth) (Class|UnWorldCharacter|GetMaxHealth))))

(event Custom|AddItem
  (params (Item :type Item%20Data%20Asset%20Object%20Reference) (ItemCount :type Integer))
  (bind _bchanged (Default|AddInventoryItem (Variables|Default|GetBpc_Inventory) Item ItemCount true))
  (Development|PrintString (select _bchanged "添加道具成功" "添加道具失败")))

(event Custom|SimpleAttack
  (Animation|Montage|PlayMontage (Variables|Character|GetMesh) "/Game/unWorld/Character/Animations/DoubleSwordStance/NormalAttack01_DoubleSwordAnim_Montage.NormalAttack01_DoubleSwordAnim_Montage"))

(event Custom|NormalAttack
  (CallFunction|DoMeleeAttack))

(event Custom|DoRoll
  (if (CallFunction|CanUseAnyAbility)
    (if (> (Math|Vector|VectorLength (Math|Vector|MakeVector (Input|AxisValues|GetMoveForward) (Input|AxisValues|GetMoveRight) 0.0)) 0.0)
      (Transformation|SetActorRotation (Pawn|GetControlRotation :!class /Script/Engine.Pawn) true))
    (CallFunction|PlayHighPriorityMontage "/Game/unWorld/Character/Animations/NoWeaponStance/Roll_noWeaponAnim_Montage.Roll_noWeaponAnim_Montage" "None")))

(event EventBeginPlay
  (Class|SkinnedMeshComponent|SetMasterPoseComponent (Variables|Default|GetHair) (Variables|Character|GetMesh) false)
  (Utilities|FlowControl|Sequence
    (:then_0
      (bind _returnvalue (UserInterface|CreateWidget "/Game/unWorld/Widgets/W_MainHUD.W_MainHUD_C"))
      (bind _output_get (Variables|Default|SetW_MainHUD _returnvalue))
      (UserInterface|Viewport|AddtoViewport _output_get 0)
      (CallFunction|UpdateHealthBar))
    (:then_1
      (Default|SetInventorySlotCount (Variables|Default|GetBpc_Inventory) 20))))

(event EventOnHealthChanged
  (params (DeltaValue :type Float%20%28single-precision%29) (EventTags :type Gameplay%20Tag%20Container%20Structure%20%28by%20ref%29))
  (CallFunction|UpdateHealthBar))

(event EventTick
  (params (DeltaSeconds :type Float%20%28single-precision%29)))

(event Input|KeyboardEvents|Q
  (params (Key :type Key%20Structure :default "None"))
  (:Pressed
    (bind _returnvalue (Abilities|TryActivateAbilitybyClass (Variables|Default|GetAbilitySystemComponent) "/Game/unWorld/Abilities/GA_DamageBase.GA_DamageBase_C" true))
    (if _returnvalue
      (Development|PrintString "q")
      (else
        (Development|PrintString "not")))))

(fn ConstructionScript)

(fn ChangeWeapon
  (params (weaponActor :type BP%20Weapon%20Base%20Class%20Reference))
  (Utilities|IsValid (Variables|Default|GetCurrentWeapon)
    (:Is%20Valid
      (Utilities|Array|RemoveItem (Variables|Default|GetGameplayAbilities) (Variables|/Game/unWorld/Blueprints/Weapon/BP_WeaponBase.BP_WeaponBase_C|GetAttackAbility (Variables|Default|GetCurrentWeapon)))
      (Actor|DestroyActor (Variables|Default|GetCurrentWeapon))
      (Variables|Default|SetCurrentWeapon 0))
    (:Is%20Not%20Valid
      _))
  (bind _returnvalue (Game|SpawnActorfromClass weaponActor (Math|Transform|MakeTransform "0, 0, 0") "AlwaysSpawn" 0 0))
  (Transformation|AttachComponentToComponent (Variables|/Script/Engine.Actor|GetRootComponent _returnvalue) (Variables|Character|GetMesh) (Variables|/Game/unWorld/Blueprints/Weapon/BP_WeaponBase.BP_WeaponBase_C|GetWeaponSocketName _returnvalue) "KeepRelative" "KeepRelative" "KeepRelative" true)
  (Variables|Default|SetEWeaponType (Variables|/Game/unWorld/Blueprints/Weapon/BP_WeaponBase.BP_WeaponBase_C|GetEWeaponType _returnvalue))
  (bind _output_get (Variables|Default|SetCurrentWeapon _returnvalue))
  (Utilities|Array|Add (Variables|Default|GetGameplayAbilities) (Variables|/Game/unWorld/Blueprints/Weapon/BP_WeaponBase.BP_WeaponBase_C|GetAttackAbility _output_get)))

(fn DoMeleeAttack
  (if (CallFunction|CanUseAnyAbility)
    (if (CallFunction|IsUsingMelee)
      _)))