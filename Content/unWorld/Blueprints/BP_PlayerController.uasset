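; BP_PlayerController is the player controller that routes input to the player character and manages HUD widgets.
; Roll and Attack inputs call the character's roll and normal attack, while Inventory and ChaInfo toggle the inventory and equipment widgets.
; Key 1 adds a test weapon item.
; BeginPlay spawns a BP_SelectedCube cursor, but the mouse-trace code that would snap it to the cube grid is unconnected.
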(event EventBeginPlay
  (bind _returnvalue (Game|SpawnActorfromClass "/Game/unWorld/Blueprints/BP_SelectedCube.BP_SelectedCube_C" (Math|Transform|MakeTransform "0, 0, 0") "AlwaysSpawn" 0 0))
  (Variables|Default|SetSelectCube _returnvalue))

(event EventTick
  (params (DeltaSeconds :type Float%20%28single-precision%29)))

(event Input|ActionEvents|InputActionRoll
  (params (Key :type Key%20Structure :default "None"))
  (:Pressed
    (bind _asbp_player_character (Utilities|Casting|CastToBP_PlayerCharacter (Game|Player|GetPlayerPawn 0)))
    (Default|DoRoll _asbp_player_character)))

(event Input|ActionEvents|InputActionChaInfo
  (params (Key :type Key%20Structure :default "None"))
  (:Pressed
    (Utilities|IsValid (Variables|Default|GetW_ChaInfo)
      (:Is%20Valid
        (Widget|RemovefromParent (Variables|Default|GetW_ChaInfo))
        (Variables|Default|SetW_ChaInfo 0))
      (:Is%20Not%20Valid
        (bind _returnvalue (UserInterface|CreateWidget "/InventorySystem/W_Equipment.W_Equipment_C"))
        (bind _output_get (Variables|Default|SetW_ChaInfo _returnvalue))
        (UserInterface|Viewport|AddtoViewport _output_get 0)))))

(event Input|ActionEvents|InputActionAttack
  (params (Key :type Key%20Structure :default "None"))
  (:Pressed
    (bind _asbp_player_character (Utilities|Casting|CastToBP_PlayerCharacter (Game|Player|GetPlayerPawn 0)))
    (Default|NormalAttack _asbp_player_character)))

(event Input|ActionEvents|InputActionInventory
  (params (Key :type Key%20Structure :default "None"))
  (:Pressed
    (Utilities|IsValid (Variables|Default|GetW_Inventory)
      (:Is%20Valid
        (Default|CloseInventory (Variables|Default|GetW_Inventory))
        (Variables|Default|SetW_Inventory 0))
      (:Is%20Not%20Valid
        (bind _returnvalue (UserInterface|CreateWidget "/InventorySystem/W_Inventory.W_Inventory_C"))
        (bind _output_get (Variables|Default|SetW_Inventory _returnvalue))
        (UserInterface|Viewport|AddtoViewport _output_get 0)))))

(event Input|KeyboardEvents|1
  (params (Key :type Key%20Structure :default "None"))
  (:Pressed
    (bind _asbp_player_character (Utilities|Casting|CastToBP_PlayerCharacter (Game|Player|GetPlayerPawn 0)))
    (Default|AddItem _asbp_player_character "/Game/unWorld/Item/DA_TestWeapon.DA_TestWeapon" 1)))

(fn ConstructionScript)