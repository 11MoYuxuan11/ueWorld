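; BP_WorldGenerator is a one-shot actor that generates the world's height map at startup.
; On BeginPlay, it builds a square height lookup sized by the WorldManager's WorldElements and passes it to the manager to create the terrain heights.
; It then notifies BP_WorldManager of success and destroys itself.
; GenerateNoiseHeight returns 3D simplex noise sampled at a frequency-scaled world position.
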(event EventBeginPlay
  (bind _worldmanager (Variables|Default|GetWorldManager))
  (bind _worldelements (Variables|/Script/unWorld.WorldManagerBase|GetWorldElements _worldmanager))
  (Utilities|IsValid _worldmanager
    (:Is%20Valid
      (bind _returnvalue (Class|OverworldMapFunctionLibrary|GenerateHeightMapLookup _worldelements _worldelements))
      (Class|WorldManagerBase|CreateHeightfromLookup (Variables|Default|GetWorldManager) _returnvalue)
      (bind _asbp_world_manager (Utilities|Casting|CastToBP_WorldManager (Variables|Default|GetWorldManager)))
      (Default|GeneratedSuccess _asbp_world_manager)
      (Actor|DestroyActor))))

(event Collision|EventActorBeginOverlap
  (params (OtherActor :type Actor%20Object%20Reference)))

(event EventTick
  (params (DeltaSeconds :type Float%20%28single-precision%29)))

(fn ConstructionScript)

(fn GenerateNoiseHeight
  (params (wPos :type Vector :default "0, 0, 0") (frequency :type Float%20%28single-precision%29))
  (bind (_x _y _z) (Math|Vector|BreakVector wPos))
  (bind _returnvalue (Class|SimplexNoiseBPLibrary|SimplexNoise3D (* _x frequency) (* _y frequency) (* _z frequency)))
  (return _returnvalue))